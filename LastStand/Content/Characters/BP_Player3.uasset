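; BP_Player3 is a player character Blueprint that configures itself from a character data input.
; BeginPlay adds IMC_Player1 to player controller 0's Enhanced Input subsystem and prints its own controller's name.
; LoadData stores the data, swaps the skeletal mesh, grants the special ability through the Ability System Component, and sets player health.
; The IA_P2 move and jump input events are empty.
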(event Input|EnhancedActionEvents|EnhancedInputActionIA_P2_Move
  (params (ActionValue :type Vector%202D%20Structure) (ElapsedSeconds :type Float%20%28double-precision%29) (TriggeredSeconds :type Float%20%28double-precision%29) (InputAction :type Input%20Action%20Object%20Reference :default "/Game/Inputs/IA_P2_Move.IA_P2_Move")))

(event Input|EnhancedActionEvents|EnhancedInputActionIA_P2_Jump
  (params (ActionValue :type Boolean) (ElapsedSeconds :type Float%20%28double-precision%29) (TriggeredSeconds :type Float%20%28double-precision%29) (InputAction :type Input%20Action%20Object%20Reference :default "/Game/Inputs/IA_P2_Jump.IA_P2_Jump")))

(event EventBeginPlay
  (Input|AddMappingContext (PlayerController|LocalPlayerSubsystems|GetEnhancedInputLocalPlayerSubsystem (Game|GetPlayerController 0)) "/Game/Inputs/IMC_Player1.IMC_Player1" 0 "(bIgnoreAllPressedKeysUntilRelease=True,bForceImmediately=False,bNotifyUserSettings=False)")
  (Development|PrintString (Utilities|GetDisplayName (Pawn|GetController))))

(event Collision|EventActorBeginOverlap
  (params (OtherActor :type Actor%20Object%20Reference)))

(event EventTick
  (params (DeltaSeconds :type Float%20%28single-precision%29)))

(fn ConstructionScript)

(fn LoadData
  (params (Data :type Character%20Data%20Object%20Reference))
  (bind _characterdata (Variables|Default|GetCharacterData))
  (bind _specialability (Variables|/Script/LastStand.CharacterData|GetSpecialAbility _characterdata))
  (Class|BasePlayer2|SetCharacterData Data)
  (Components|SkeletalMesh|SetSkeletalMeshAsset (Variables|Character|GetMesh) (Variables|/Script/LastStand.CharacterData|GetSkeletalMesh Data))
  (bind _returnvalue (GameplayAbilities|GiveAbility (Variables|Default|GetAbilitySystemComponent) _specialability 0 -1))
  (Development|PrintString (Utilities|GetClassDisplayName _specialability))
  (Variables|Default|SetAbility _returnvalue)
  (Variables|Default|SetPlayerHealth (Variables|/Script/LastStand.CharacterData|GetHealth Data)))