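; BP_Thunderball is a gameplay ability actor that damages specific player characters on contact.
; When its Sphere begins an overlap, it waits briefly, then checks that the other actor is not OwningActor and is tagged Player1 or Player3.
; It casts to the matching player Blueprint, calls TakeDamage with its Damage value, and destroys itself.
; Other overlapping actors take no damage and leave it alive.
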(event OnComponentBeginOverlap(Sphere)
  (params (OverlappedComponent :type Primitive%20Component%20Object%20Reference) (OtherActor :type Actor%20Object%20Reference) (OtherComp :type Primitive%20Component%20Object%20Reference) (OtherBodyIndex :type Integer) (bFromSweep :type Boolean) (SweepResult :type Hit%20Result%20Structure%20%28by%20ref%29))
  (Utilities|FlowControl|Delay 0.2)
  (if (and (!= (Variables|Default|GetOwningActor) OtherActor) (Actor|ActorHasTag OtherActor "Player1"))
    (bind _asbp_player_1 (Utilities|Casting|CastToBP_Player1 OtherActor))
    (Default|TakeDamage _asbp_player_1 (Variables|Default|GetDamage))
    (Actor|DestroyActor)
    (elif (and (!= (Variables|Default|GetOwningActor) OtherActor) (Actor|ActorHasTag OtherActor "Player3"))
      (bind _asbp_player_3 (Utilities|Casting|CastToBP_Player3 OtherActor))
      (Default|TakeDamage _asbp_player_3 (Variables|Default|GetDamage))
      (Actor|DestroyActor))))

(fn ConstructionScript)