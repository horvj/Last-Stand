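; BP_Fireball is a fireball hazard actor that eliminates a player on contact and ends the match.
; Its Sphere overlap waits briefly, then destroys the other actor if it is not OwningActor and is tagged Player1 or Player3.
; After a further delay it opens the MainMenu level.
; The file contains no movement, damage or effects logic.
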(event OnComponentBeginOverlap(Sphere)
  (params (OverlappedComponent :type Primitive%20Component%20Object%20Reference) (OtherActor :type Actor%20Object%20Reference) (OtherComp :type Primitive%20Component%20Object%20Reference) (OtherBodyIndex :type Integer) (bFromSweep :type Boolean) (SweepResult :type Hit%20Result%20Structure%20%28by%20ref%29))
  (Utilities|FlowControl|Delay 0.2)
  (if (and (!= (Variables|Default|GetOwningActor) OtherActor) (Actor|ActorHasTag OtherActor "Player1"))
    (Actor|DestroyActor OtherActor)
    (Utilities|FlowControl|Delay 1.0)
    (Game|OpenLevel(byObjectReference) "/Game/Menus/MainMenu.MainMenu")
    (elif (and (!= (Variables|Default|GetOwningActor) OtherActor) (Actor|ActorHasTag OtherActor "Player3"))
      (Actor|DestroyActor OtherActor)
      (Utilities|FlowControl|Delay 1.0)
      (Game|OpenLevel(byObjectReference) "/Game/Menus/MainMenu.MainMenu"))))

(event EventBeginPlay)

(event Collision|EventActorBeginOverlap
  (params (OtherActor :type Actor%20Object%20Reference)))

(event EventTick
  (params (DeltaSeconds :type Float%20%28single-precision%29)))

(fn ConstructionScript)