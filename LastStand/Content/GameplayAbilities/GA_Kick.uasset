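; Gameplay ability for a kick attack that spawns a temporary hit zone at the character's left foot.
; It plays the kick montage and waits for the Event.Montage.Kick gameplay event to spawn a BP_PunchZone, assigning the avatar's owner actor as its OwningActor.
; A DoOnce limits this to one zone per kick.
; Montage completion alone ends the ability and resets the gate, and ending destroys the zone.
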(event Ability|EventActivateAbility
  (bind _returnvalue (Ability|GetActorInfo))
  (|PlayMontageandWaitProxy "None" "/Game/Animations/AM_Kick.AM_Kick" 1.0 "None" true 1.0 0.0 false
    (:then
      (Ability|Tasks|WaitGameplayEvent "(TagName=\"Event.Montage.Kick\")" 0
        (:EventReceived
          (Utilities|FlowControl|DoOnce false :!label _label
            (:Completed
              (bind _returnvalue_2 (Game|SpawnActorfromClass "/Game/GameplayAbilities/BP_PunchZone.BP_PunchZone_C" (Math|Transform|MakeTransform (Transformation|GetSocketLocation (.skeletalmeshcomponent _returnvalue) "foot_l") (Transformation|GetActorRotation (.owneractor _returnvalue)) "1.000000,1.000000,1.000000") "Undefined" "MultiplyWithRoot" 0 0))
              (bind _output_get (Variables|Default|SetPunchZone _returnvalue_2))
              (Variables|/Game/GameplayAbilities/BP_PunchZone.BP_PunchZone_C|SetOwningActor _output_get (.owneractor _returnvalue)))))))
    (:OnCompleted
      (Ability|EndAbility)
      (goto _label Reset))))

(event Ability|EventOnEndAbility
  (params (bWasCancelled :type Boolean))
  (Actor|DestroyActor (Variables|Default|GetPunchZone)))