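; Player controller that handles input for both characters in a two-player game with punches and special abilities.
; Enhanced Input actions drive movement along world Y and jumping on player characters 0 and 1.
; Combat inputs find the first BP_Player1 or BP_Player3 actor and activate GAS abilities on it.
; Punches share GA_Punch, while specials come from Player 1's CharacterData and Player 2's stored Ability.
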(event Input|EnhancedActionEvents|EnhancedInputActionIA_P1_Move
  (params (ActionValue :type Vector%202D%20Structure) (ElapsedSeconds :type Float%20%28double-precision%29) (TriggeredSeconds :type Float%20%28double-precision%29) (InputAction :type Input%20Action%20Object%20Reference :default "/Game/Inputs/IA_P1_Move.IA_P1_Move"))
  (Pawn|Input|AddMovementInput (Game|GetPlayerCharacter 0) (Math|Vector|MakeVector 0.0 (.y ActionValue) 0.0) 1.0 false))

(event Input|EnhancedActionEvents|EnhancedInputActionIA_P1_Jump
  (params (ActionValue :type Boolean) (ElapsedSeconds :type Float%20%28double-precision%29) (TriggeredSeconds :type Float%20%28double-precision%29) (InputAction :type Input%20Action%20Object%20Reference :default "/Game/Inputs/IA_P1_Jump.IA_P1_Jump"))
  (if ActionValue
    (Character|Jump (Game|GetPlayerCharacter 0))))

(event Input|EnhancedActionEvents|EnhancedInputActionIA_P2_Jump
  (params (ActionValue :type Boolean) (ElapsedSeconds :type Float%20%28double-precision%29) (TriggeredSeconds :type Float%20%28double-precision%29) (InputAction :type Input%20Action%20Object%20Reference :default "/Game/Inputs/IA_P2_Jump.IA_P2_Jump"))
  (if ActionValue
    (Character|Jump (Game|GetPlayerCharacter 1))))

(event Input|EnhancedActionEvents|EnhancedInputActionIA_P2_Move
  (params (ActionValue :type Vector%202D%20Structure) (ElapsedSeconds :type Float%20%28double-precision%29) (TriggeredSeconds :type Float%20%28double-precision%29) (InputAction :type Input%20Action%20Object%20Reference :default "/Game/Inputs/IA_P2_Move.IA_P2_Move"))
  (Pawn|Input|AddMovementInput (Game|GetPlayerCharacter 1) (Math|Vector|MakeVector 0.0 (.x ActionValue) 0.0) -1.0 false))

(event Input|EnhancedActionEvents|EnhancedInputActionIA_P2_Special_Ability
  (params (ActionValue :type Boolean) (ElapsedSeconds :type Float%20%28double-precision%29) (TriggeredSeconds :type Float%20%28double-precision%29) (InputAction :type Input%20Action%20Object%20Reference :default "/Game/Inputs/IA_P2_Special_Ability.IA_P2_Special_Ability"))
  (bind _outactors (Actor|GetAllActorsOfClass "/Game/Characters/BP_Player3.BP_Player3_C"))
  (Class|AbilitySystemComponent|TryActivateAbility (Variables|/Script/LastStand.BasePlayer2|GetAbilitySystemComponent (Utilities|Array|Get(acopy) _outactors)) (Variables|/Game/Characters/BP_Player3.BP_Player3_C|GetAbility (Utilities|Array|Get(acopy) _outactors)) true))

(event Input|EnhancedActionEvents|EnhancedInputActionIA_P1_Special_Ability
  (params (ActionValue :type Boolean) (ElapsedSeconds :type Float%20%28double-precision%29) (TriggeredSeconds :type Float%20%28double-precision%29) (InputAction :type Input%20Action%20Object%20Reference :default "/Game/Inputs/IA_P1_Special_Ability.IA_P1_Special_Ability"))
  (bind _outactors (Actor|GetAllActorsOfClass "/Game/Characters/BP_Player1.BP_Player1_C"))
  (Abilities|TryActivateAbilitybyClass (Variables|/Script/LastStand.BasePlayer1|GetAbilitySystemComponent (Utilities|Array|Get(acopy) _outactors)) (Variables|/Script/LastStand.CharacterData|GetSpecialAbility (Variables|/Script/LastStand.BasePlayer1|GetCharacterData (Utilities|Array|Get(acopy) _outactors))) true))

(event Input|EnhancedActionEvents|EnhancedInputActionIA_P2_Punch
  (params (ActionValue :type Boolean) (ElapsedSeconds :type Float%20%28double-precision%29) (TriggeredSeconds :type Float%20%28double-precision%29) (InputAction :type Input%20Action%20Object%20Reference :default "/Game/Inputs/IA_P2_Punch.IA_P2_Punch"))
  (:Triggered
    (bind _outactors (Actor|GetAllActorsOfClass "/Game/Characters/BP_Player3.BP_Player3_C"))
    (Utilities|FlowControl|DoOnce false :!label _label
      (:Completed
        (Abilities|TryActivateAbilitybyClass (Variables|/Script/LastStand.BasePlayer2|GetAbilitySystemComponent (Utilities|Array|Get(acopy) _outactors)) "/Game/GameplayAbilities/GA_Punch.GA_Punch_C" true)
        (goto _label Reset)))))

(event Input|EnhancedActionEvents|EnhancedInputActionIA_P2_Kick
  (params (ActionValue :type Boolean) (ElapsedSeconds :type Float%20%28double-precision%29) (TriggeredSeconds :type Float%20%28double-precision%29) (InputAction :type Input%20Action%20Object%20Reference :default "/Game/Inputs/IA_P2_Kick.IA_P2_Kick")))

(event Input|EnhancedActionEvents|EnhancedInputActionIA_P1_Punch
  (params (ActionValue :type Boolean) (ElapsedSeconds :type Float%20%28double-precision%29) (TriggeredSeconds :type Float%20%28double-precision%29) (InputAction :type Input%20Action%20Object%20Reference :default "/Game/Inputs/IA_P1_Punch.IA_P1_Punch"))
  (bind _outactors (Actor|GetAllActorsOfClass "/Game/Characters/BP_Player1.BP_Player1_C"))
  (Utilities|FlowControl|DoOnce false :!label _label
    (:Completed
      (Abilities|TryActivateAbilitybyClass (Ability|GetAbilitySystemComponent (Utilities|Array|Get(acopy) _outactors)) "/Game/GameplayAbilities/GA_Punch.GA_Punch_C" true)
      (goto _label Reset))))

(event EventBeginPlay
  (Utilities|FlowControl|Delay 0.2)
  (Variables|Default|SetPlayer2 (Game|GetPlayerCharacter 1)))

(event EventTick
  (params (DeltaSeconds :type Float%20%28single-precision%29)))

(fn ConstructionScript)